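; AC_Listener is an actor component that activates or deactivates its owner based on how many connected activators are currently on.
; Each connected activator raises the required count unless a custom amount overrides it, while activation and deactivation requests adjust the current count.
; The owner counts as active when all required or at least one activation is present, depending on a flag.
; Every request forwards the result to the owner through BI_Listener, logging if that interface is missing.
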(event Custom|Request%20Deactivation
  (bind _returnvalue (Components|GetOwner))
  (Variables|Default|SetActivationCurrentAmount (- (Variables|Default|GetActivationCurrentAmount) 1))
  (bind _activationstatus (CallFunction|CheckActivationRequirements))
  (Variables|Default|SetIsActivated _activationstatus)
  (if (Utilities|DoesObjectImplementInterface _returnvalue "/Game/_TinyIslands/Actors/Ingredients/Modules/BI_Listener.BI_Listener_C")
    (bind _asbi_listener (Utilities|Casting|CastToBI_Listener _returnvalue))
    (if (Variables|Default|GetIsActivated)
      (Default|ActivateListener _asbi_listener)
      (else
        (Default|DeactivateListener _asbi_listener)))
    (else
      (Utilities|String|LogString "AC_Listener : Parent does not implement BI_Listener interface"))))

(event Custom|Request%20Activation
  (bind _returnvalue (Components|GetOwner))
  (Variables|Default|SetActivationCurrentAmount (+ (Variables|Default|GetActivationCurrentAmount) 1))
  (bind _activationstatus (CallFunction|CheckActivationRequirements))
  (Variables|Default|SetIsActivated _activationstatus)
  (if (Utilities|DoesObjectImplementInterface _returnvalue "/Game/_TinyIslands/Actors/Ingredients/Modules/BI_Listener.BI_Listener_C")
    (bind _asbi_listener (Utilities|Casting|CastToBI_Listener _returnvalue))
    (if (Variables|Default|GetIsActivated)
      (Default|ActivateListener _asbi_listener)
      (else
        (Default|DeactivateListener _asbi_listener)))
    (else
      (Utilities|String|LogString "AC_Listener : Parent does not implement BI_Listener interface"))))

(event Custom|Add%20Connected%20Activator
  (if (== (Variables|Default|GetCustomRequiredAmount) 0)
    (Variables|Default|SetActivationRequieredAmount (+ (Variables|Default|GetActivationRequieredAmount) 1))
    (else
      (Variables|Default|SetActivationRequieredAmount (Variables|Default|GetCustomRequiredAmount)))))

(event EventBeginPlay)

(event EventTick
  (params (DeltaSeconds :type Float%20%28single-precision%29)))

(fn CheckActivationRequirements
  (if (Variables|Default|GetRequiresAllActivated)
    (LocalVariables|SetActivated (>= (Variables|Default|GetActivationCurrentAmount) (Variables|Default|GetActivationRequieredAmount)))
    (else
      (LocalVariables|SetActivated (>= (Variables|Default|GetActivationCurrentAmount) 1))))
  (return (LocalVariables|GetActivated) false))

(fn UpdateActivationStatus)